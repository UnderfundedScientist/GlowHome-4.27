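; GoldCowBP is a short-lived gold cow prop that tumbles through a RotatingMovement component.
; The construction script gives it a fixed starting orientation and a random spin rate, clamping each axis to a limited non-negative range.
; On BeginPlay a one-shot timer, stored in DespawnHandle, destroys the actor after 15 seconds.
; A node setting the mesh material's Glow parameter is present but never runs.
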(event `self.ReceiveBeginPlay`
  (`|ExecutionSequence`
    (:`then_1`
      (bind _returnvalue (`KismetSystemLibrary.K2_SetTimerDelegate` (delegate `Despawn`) 15.0))
      (set `self.DespawnHandle` _returnvalue))))

(event `Despawn`
  (`self.K2_DestroyActor`))

(fn `UserConstructionScript`
  (bind (_returnvalue_roll _returnvalue_pitch _returnvalue_yaw) (`KismetMathLibrary.BreakRotator` (`KismetMathLibrary.RandomRotator` true)))
  (`self.K2_SetActorRotation` (struct :`Roll` 90.0))
  (set `RotatingMovementComponent.RotationRate` (`KismetMathLibrary.MakeRotator` (`KismetMathLibrary.FClamp` _returnvalue_roll 0.0 70.0) (`KismetMathLibrary.FClamp` _returnvalue_pitch 0.0 70.0) (`KismetMathLibrary.FClamp` _returnvalue_yaw 0.0 70.0)) (`self.RotatingMovement`)))