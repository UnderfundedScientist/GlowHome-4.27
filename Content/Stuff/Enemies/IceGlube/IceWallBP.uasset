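; IceWallBP is a short-lived ice wall hazard, filed under the IceGlube enemy, that damages the player on hit.
; On BeginPlay it scales its mesh up along a timeline curve, caches the game instance and destroys itself after two seconds.
; A gated Hit on TwinStickPawn subtracts a fraction of max health from the game instance.
; At zero health it triggers player death, saves, then after a delay opens DeathScreen.
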(event `self.CollisionSphere.OnComponentHit`
  (params (HitComponent :type "PrimitiveComponent Object Reference") (OtherActor :type "Actor Object Reference") (OtherComp :type "PrimitiveComponent Object Reference") (NormalImpulse :type "Vector Structure") (Hit :type "HitResult Structure (by ref)")))

(event `self.ReceiveBeginPlay`
  (`|ExecutionSequence`
    (:`then_0`
      (bind (_direction _newtrack_0) (`Timeline|IceWallGrowthCurve`)
        (:`Update`
          (`SceneComponent.SetWorldScale3D` (`self.IceWallMesh`) (`KismetMathLibrary.VLerp` (1.0 1.0 1.0) (5.0 5.0 5.0) _newtrack_0)))))
    (:`then_1`
      (bind _asinstance_player_0 (cast `/Game/Stuff/Instance/InstancePlayer0` (`GameplayStatics.GetGameInstance`)))
      (set `self.Instance` _asinstance_player_0))
    (:`then_2`
      (`KismetSystemLibrary.Delay` 2.0)
      (`self.K2_DestroyActor`))))

(event `self.ReceiveHit`
  (params (MyComp :type "PrimitiveComponent Object Reference") (Other :type "Actor Object Reference") (OtherComp :type "PrimitiveComponent Object Reference") (bSelfMoved :type Boolean) (HitLocation :type "Vector Structure") (HitNormal :type "Vector Structure") (NormalImpulse :type "Vector Structure") (Hit :type "HitResult Structure (by ref)"))
  (bind _instance (`self.Instance`))
  (bind _playerhealthmaxinstance (`/Game/Stuff/Instance/InstancePlayer0.PlayerHealthMaxInstance` _instance))
  (bind _astwin_stick_pawn (cast `/Game/Stuff/TwinStickBP/Blueprints/TwinStickPawn` Other))
  (if (== _astwin_stick_pawn Other)
    (`/Engine/EditorBlueprintResources/StandardMacros.DoOnce` false :!label _label
      (:`Completed`
        (bind _output_get (set `/Game/Stuff/Instance/InstancePlayer0.PlayerHealthInstance` (- (`/Game/Stuff/Instance/InstancePlayer0.PlayerHealthInstance` _instance) (* _playerhealthmaxinstance 0.05)) _instance))
        (set `/Game/Stuff/Instance/InstancePlayer0.PlayerHealthPercentInstance` (/ _output_get _playerhealthmaxinstance) _instance)
        (if (<= _output_get 0.0)
          (`/Engine/EditorBlueprintResources/StandardMacros.DoOnce` false
            (:`Completed`
              (`/Game/Stuff/TwinStickBP/Blueprints/TwinStickPawn.PlayerDeath` _astwin_stick_pawn)
              (`/Game/Stuff/Instance/InstancePlayer0.SavePlayerData` _instance)
              (`KismetSystemLibrary.Delay` 1.5)
              (set `/Game/Stuff/Instance/InstancePlayer0.CanBeDamagedInstance` false _instance)
              (`GameplayStatics.OpenLevel` "DeathScreen")))
          (else
            (`KismetSystemLibrary.Delay` 2.0)
            (goto _label :!via `Reset`)))))))

(fn `UserConstructionScript`)