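; Meat enemy for a twin-stick game that chases the player through a self-repeating AIMoveTo.
; Hit casts the other actor to apply cannon, missile, plasma or asteroid damage from game-instance stats, with floating numbers and light blinks.
; Player and asteroid contacts knock it back; plasma damage has a cooldown.
; Death awards XP and gold, updates enemy population, and rolls for pickups or a half-scale enemy spawn.
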(event `self.PawnSensing.OnHearNoise`
  (params (Instigator :type "Pawn Object Reference") (Location :type "Vector Structure (by ref)") (Volume :type "Float (single-precision)")))

(event `CastEvent`
  (`|ExecutionSequence`
    (:`then_0`
      (bind _asinstance_player_0 (cast `/Game/Stuff/Instance/InstancePlayer0` (`GameplayStatics.GetGameInstance`)))
      (set `self.InstancePlayer0` _asinstance_player_0))
    (:`then_1`
      ;[1 1 1] AssignUI
      (bind _asmeat_ui (cast `/Game/Stuff/Enemies/Meat/MeatUi` (`WidgetComponent.GetUserWidgetObject` (`self.EnemyHealthWidget`))))
      (set `/Game/Stuff/Enemies/Meat/MeatUi.MeatBp` self _asmeat_ui))
    (:`then_2`
      (bind _astwin_stick_pawn (cast `/Game/Stuff/TwinStickBP/Blueprints/TwinStickPawn` (`GameplayStatics.GetPlayerPawn` 0)))
      (set `self.Player` _astwin_stick_pawn))))

(event `self.ReceiveTick`
  (params (DeltaSeconds :type "Float (single-precision)")))

(event `self.PawnSensing.OnSeePawn`
  (params (Pawn :type "Pawn Object Reference"))
  (`|AIMoveTo` self (0.0 0.0 0.0) (`GameplayStatics.GetPlayerPawn` 0) 0.0))

(event `AttackCooldown`
  (set `self.CanAttack` true))

(event `DamageCooldown`
  (set `self.PlasmaCanDamage` true))

(event `self.ReceiveBeginPlay`
  (`|ExecutionSequence`
    (:`then_0`
      (`self.CastEvent`))
    (:`then_1`
      (`SkeletalMeshComponent.PlayAnimation` (`self.Mesh`) "/Game/Stuff/Enemies/Meat/MeatRig_Anim.MeatRig_Anim" true))
    (:`then_3`
      (bind _output_get (set `self.CurrentHealth` (* (`/Game/Stuff/Instance/InstancePlayer0.EnemyOneHealthMax` (`self.InstancePlayer0`)) 3.0)))
      (set `self.MaxHealth` _output_get)
      (set `self.HealthPercentEnemyOne` (/ (`self.CurrentHealth`) (`self.MaxHealth`))))
    (:`then_4`
      (`KismetSystemLibrary.Delay` 3.0)
      (`self.LockOnPlayer`))
    (:`then_5`)))

(event `LockOnPlayer`
  (`self.K2_SetActorRotation` (`KismetMathLibrary.Conv_VectorToRotator` (`KismetMathLibrary.GetDirectionUnitVector` (`self.K2_GetActorLocation`) (`self.K2_GetActorLocation` (`GameplayStatics.GetPlayerPawn` 0)))))
  (`|AIMoveTo` self (0.0 0.0 0.0) (`GameplayStatics.GetPlayerPawn` 0) 0.0
    (:`OnSuccess`
      _)
    (:`OnFail`
      _))
  (`self.LockOnPlayer`))

(event `PlasmaDamageReset`
  ;[1 1 1] PlasmaDamageReset
  (set `self.PlasmaCanDamage` true))

(event `DeathEvent`
  (bind _instanceplayer0 (`self.InstancePlayer0`))
  (bind _instanceplayer0_2 (`self.InstancePlayer0`))
  (bind _missile (`self.Missile`))
  ;[1 1 1] DeathEvent
  (`|ExecutionSequence`
    (:`then_0`
      (set `/Game/Stuff/Instance/InstancePlayer0.XpCurrentInstance` (+ (`/Game/Stuff/Instance/InstancePlayer0.XpCurrentInstance` _instanceplayer0_2) (`/Game/Stuff/Instance/InstancePlayer0.RewardXp` _instanceplayer0_2)) _instanceplayer0_2)
      (`/Game/Stuff/TwinStickBP/Blueprints/TwinStickPawn.AddXP` (`self.Player`)))
    (:`then_1`
      (set `/Game/Stuff/Instance/InstancePlayer0.GoldInstance` (+ (`/Game/Stuff/Instance/InstancePlayer0.GoldInstance` _instanceplayer0) (`/Game/Stuff/Instance/InstancePlayer0.RewardGold` _instanceplayer0)) _instanceplayer0))
    (:`then_2`
      (bind _astwin_stick_pawn (cast `/Game/Stuff/TwinStickBP/Blueprints/TwinStickPawn` (`GameplayStatics.GetPlayerPawn` 0)))
      (set `/Game/Stuff/TwinStickBP/Blueprints/TwinStickPawn.EnemyPopulation` (- (`/Game/Stuff/TwinStickBP/Blueprints/TwinStickPawn.EnemyPopulation` _astwin_stick_pawn) 1.0) _astwin_stick_pawn))
    (:`then_3`
      (`GameplayStatics.SpawnEmitterAtLocation` "/Game/MobileStarterContent/Particles/P_Explosion.P_Explosion" (`self.K2_GetActorLocation`) (struct) (3.0 3.0 3.0))
      (`NiagaraFunctionLibrary.SpawnSystemAtLocation` "/Game/Stuff/Particles/EnemyDeathSystem.EnemyDeathSystem" (`self.K2_GetActorLocation`) (struct) (3.0 3.0 3.0))
      (`GameplayStatics.PlaySoundAtLocation` "/Game/MobileStarterContent/Audio/Explosion02.Explosion02" (0.0 0.0 0.0) (struct) 0.125 (`KismetMathLibrary.RandomFloatInRange` -1.0 0.3) 0.0 null null null))
    (:`then_4`
      (`self.RollForDrops`))
    (:`then_5`
      (`/Engine/EditorBlueprintResources/StandardMacros.IsValid` _missile
        (:`Is Valid`
          (`/Game/Stuff/Projectiles/Missile.StartHoming` _missile))))
    (:`then_6`
      (`self.K2_DestroyActor`))))

(event `self.ReceiveHit`
  (params (MyComp :type "PrimitiveComponent Object Reference") (Other :type "Actor Object Reference") (OtherComp :type "PrimitiveComponent Object Reference") (bSelfMoved :type Boolean) (HitLocation :type "Vector Structure") (HitNormal :type "Vector Structure") (NormalImpulse :type "Vector Structure") (Hit :type "HitResult Structure (by ref)"))
  (bind _pointlight (`self.PointLight`))
  (bind _pointlight_2 (`self.PointLight`))
  (bind _pointlight_3 (`self.PointLight`))
  (bind _pointlight_4 (`self.PointLight`))
  (bind _pointlight_5 (`self.PointLight`))
  (`|ExecutionSequence`
    (:`then_0`
      (bind _astwin_stick_projectile (cast `/Game/Stuff/TwinStickBP/Blueprints/TwinStickProjectile` Other))
      (if (== _astwin_stick_projectile Other)
        ;[1 1 1] CannonHit
        (`self.CannonDamageEvent` HitLocation)
        (`LightComponent.SetIntensity` _pointlight_2 0.0)
        (`KismetSystemLibrary.Delay` 0.2)
        (`LightComponent.SetIntensity` _pointlight_2 400000.0)
        (if (<= (`self.CurrentHealth`) 0.0)
          (`self.DeathEvent`))))
    (:`then_1`
      (bind _astwin_stick_pawn (cast `/Game/Stuff/TwinStickBP/Blueprints/TwinStickPawn` Other))
      ;[1 1 1] MeleeHitPlayer
      (if (== _astwin_stick_pawn Other)
        (bind _output_get (`self.CalculateLaunchVelocity` (`self.Player`)))
        (`self.LaunchCharacter` _output_get)
        (`LightComponent.SetIntensity` _pointlight_3 0.0)
        (`KismetSystemLibrary.Delay` 0.2)
        (`LightComponent.SetIntensity` _pointlight_3 400000.0)))
    (:`then_2`
      ;[1 1 1] MissileHit
      (bind _asmissile (cast `/Game/Stuff/Projectiles/Missile` Other))
      (if (== _asmissile Other)
        (`self.MissileDamageEvent` HitLocation)
        (`LightComponent.SetIntensity` _pointlight_4 0.0)
        (`KismetSystemLibrary.Delay` 0.2)
        (`LightComponent.SetIntensity` _pointlight_4 400000.0)
        (if (<= (`self.CurrentHealth`) 0.0)
          (`self.DeathEvent`))))
    (:`then_3`
      ;[1 1 1] PlasmaHit
      (bind _asplasma_projectile (cast `/Game/Stuff/Projectiles/PlasmaProjectile` Other))
      (if (and (== _asplasma_projectile Other) (`self.PlasmaCanDamage`))
        (set `self.PlasmaMostRecentHit` _asplasma_projectile)
        (set `self.PlasmaCanDamage` false)
        (`KismetSystemLibrary.K2_SetTimer` null "PlasmaDamageReset" 3.0)
        (`self.PlasmaDamageEvent` HitLocation)
        (`LightComponent.SetIntensity` _pointlight_5 0.0)
        (`KismetSystemLibrary.Delay` 0.2)
        (`LightComponent.SetIntensity` _pointlight_5 400000.0)
        (if (<= (`self.CurrentHealth`) 0.0)
          (`self.DeathEvent`))))
    (:`then_4`
      ;[1 1 1] AsteroidHit
      (bind _asasteroid_spherical (cast `/Game/Stuff/Asteroid/AsteroidSpherical` Other))
      (if (and (== _asasteroid_spherical Other) (`self.ActorHasTag` _asasteroid_spherical "Asteroid") (`/Game/Stuff/TwinStickBP/Blueprints/TwinStickPawn.Attached` (`self.Player`)))
        (`self.AsteroidDamageEvent` HitLocation)
        (bind _output_get_2 (`self.CalculateLaunchVelocity` _asasteroid_spherical))
        (`self.LaunchCharacter` _output_get_2)
        (`LightComponent.SetIntensity` _pointlight 0.0)
        (`KismetSystemLibrary.Delay` 0.2)
        (`LightComponent.SetIntensity` _pointlight 400000.0)
        (`KismetSystemLibrary.Delay` 2.0)
        (`self.LockOnPlayer`)
        (if (<= (`self.CurrentHealth`) 0.0)
          (`self.DeathEvent`))))
    (:`then_5`
      (`KismetSystemLibrary.Delay` 0.2)
      (`self.LockOnPlayer`))))

(event `self.ReceiveActorBeginOverlap`
  (params (OtherActor :type "Actor Object Reference")))

(event `CannonDamageEvent`
  (params (HitLocation :type "Vector Structure"))
  (bind _returnvalue (* (`/Game/Stuff/Instance/InstancePlayer0.CannonDamage` (`self.InstancePlayer0`)) 2.0))
  ;[1 1 1] CannonDamageEvent
  (`NiagaraFunctionLibrary.SpawnSystemAtLocation` "/Game/Stuff/Particles/CannonCollision_System.CannonCollision_System" HitLocation (struct) (2.0 2.0 2.0))
  (`GameplayStatics.PlaySoundAtLocation` "/Game/TwinStick/Audio/TwinStickFire.TwinStickFire" HitLocation (struct) 0.2 (`KismetMathLibrary.RandomFloatInRange` -4.0 4.0) 0.0 null null null)
  (if (>= (`KismetMathLibrary.RandomIntegerInRange` 1 10) 9)
    (bind _output_get (set `self.CurrentHealth` (- (`self.CurrentHealth`) _returnvalue)))
    (set `self.HealthPercentEnemyOne` (/ _output_get (`self.MaxHealth`)))
    (bind _returnvalue_2 (`|SpawnActorFromClass` "/Game/Stuff/UI/CannonDamageUIBP.CannonDamageUIBP_C" (`KismetMathLibrary.MakeTransform` (+ HitLocation (`KismetMathLibrary.MakeVector` (`KismetMathLibrary.RandomFloatInRange` -200.0 200.0) (`KismetMathLibrary.RandomFloatInRange` -200.0 200.0) 200.0))) "Undefined" "OverrideRootScale" null null))
    (bind _ascannon_damage_ui (cast `/Game/Stuff/UI/CannonDamageUI` (`WidgetComponent.GetUserWidgetObject` (`/Game/Stuff/UI/CannonDamageUIBP.Widget` _returnvalue_2))))
    (`TextBlock.SetText` (`/Game/Stuff/UI/CannonDamageUI.DamageText` _ascannon_damage_ui) (`KismetTextLibrary.Conv_DoubleToText` _returnvalue "HalfToEven"))
    (else
      (bind _output_get_2 (set `self.CurrentHealth` (- (`self.CurrentHealth`) (`/Game/Stuff/Instance/InstancePlayer0.CannonDamage` (`self.InstancePlayer0`)))))
      (set `self.HealthPercentEnemyOne` (/ _output_get_2 (`self.MaxHealth`)))
      (bind _returnvalue_3 (`|SpawnActorFromClass` "/Game/Stuff/UI/CannonDamageUIBP.CannonDamageUIBP_C" (`KismetMathLibrary.MakeTransform` (+ HitLocation (`KismetMathLibrary.MakeVector` (`KismetMathLibrary.RandomFloatInRange` -200.0 200.0) (`KismetMathLibrary.RandomFloatInRange` -200.0 200.0) 200.0))) "Undefined" "OverrideRootScale" null null))
      (bind _ascannon_damage_ui_2 (cast `/Game/Stuff/UI/CannonDamageUI` (`WidgetComponent.GetUserWidgetObject` (`/Game/Stuff/UI/CannonDamageUIBP.Widget` _returnvalue_3))))
      (`TextBlock.SetText` (`/Game/Stuff/UI/CannonDamageUI.DamageText` _ascannon_damage_ui_2) (`KismetTextLibrary.Conv_DoubleToText` (`/Game/Stuff/Instance/InstancePlayer0.CannonDamage` (`self.InstancePlayer0`)) "HalfToEven")))))

(event `RollForDrops`
  (bind _returnvalue_x (`KismetMathLibrary.BreakVector` (`self.GetActorScale3D`)))
  (bind _player (`self.Player`))
  (bind _randomlocation (`NavigationSystemV1.K2_GetRandomLocationInNavigableRadius` (`self.K2_GetActorLocation`) 700.0 null null))
  (bind _randomlocation_2 (`NavigationSystemV1.K2_GetRandomLocationInNavigableRadius` (`self.K2_GetActorLocation`) 700.0 null null))
  (bind _randomlocation_3 (`NavigationSystemV1.K2_GetRandomLocationInNavigableRadius` (`self.K2_GetActorLocation`) 700.0 null null))
  (bind _randomlocation_4 (`NavigationSystemV1.K2_GetRandomLocationInNavigableRadius` (`self.K2_GetActorLocation`) 700.0 null null))
  (bind _enemyarray (`/Game/Stuff/Instance/InstancePlayer0.EnemyArray` (`self.InstancePlayer0`)))
  ;[1 1 1] RollForDrops
  (`|ExecutionSequence`
    (:`then_0`
      ;;[1 1 1] SmallEnemySpawn
      (if (and (>= (`KismetMathLibrary.RandomIntegerInRange` 1 10) 3) (> _returnvalue_x 0.6))
        (bind _returnvalue (`AIBlueprintHelperLibrary.SpawnAIFromClass` (`|GetArrayItem` _enemyarray (`KismetMathLibrary.RandomIntegerInRange` 0 (`KismetArrayLibrary.Array_LastIndex` _enemyarray))) null (`KismetMathLibrary.MakeVector` (.x _randomlocation_2) (.y _randomlocation_2) (+ (.z _randomlocation_2) 200.0)) (struct) false null))
        (`self.SetActorScale3D` _returnvalue (/ (`self.GetActorScale3D` _returnvalue) 2.0))
        (set `/Game/Stuff/TwinStickBP/Blueprints/TwinStickPawn.EnemyPopulation` (+ (`/Game/Stuff/TwinStickBP/Blueprints/TwinStickPawn.EnemyPopulation` _player) 1.0) _player)))
    (:`then_1`
      ;;[1 1 1] GoldCowSpawn
      (if (>= (`KismetMathLibrary.RandomIntegerInRange` 1 10) 9)
        (`|SpawnActorFromClass` "/Game/Stuff/Props/GoldCowBP.GoldCowBP_C" (`KismetMathLibrary.MakeTransform` (`KismetMathLibrary.MakeVector` (.x _randomlocation_4) (.y _randomlocation_4) (+ (.z _randomlocation_4) 200.0)) (struct) (400.0 400.0 400.0)) "Undefined" "OverrideRootScale" null null)))
    (:`then_2`
      ;;[1 1 1] SpwnHeartDrop
      (if (>= (`KismetMathLibrary.RandomIntegerInRange` 1 10) 9)
        (`|SpawnActorFromClass` "/Game/Stuff/Drops/HealthDrop/HeartBp.HeartBp_C" (`KismetMathLibrary.MakeTransform` (`KismetMathLibrary.MakeVector` (.x _randomlocation) (.y _randomlocation) (+ (.z _randomlocation) 200.0))) "Undefined" "OverrideRootScale" null null)))
    (:`then_3`
      (if (>= (`KismetMathLibrary.RandomIntegerInRange` 1 20) 20)
        (`|SpawnActorFromClass` "/Game/Stuff/Drops/BrainChooseYourFate/BrainBP.BrainBP_C" (`KismetMathLibrary.MakeTransform` (`KismetMathLibrary.MakeVector` (.x _randomlocation_3) (.y _randomlocation_3) (+ (.z _randomlocation_3) 200.0))) "Undefined" "OverrideRootScale" null null)))))

(event `MissileDamageEvent`
  (params (HitLocation :type "Vector Structure"))
  (bind _returnvalue (* (`/Game/Stuff/Instance/InstancePlayer0.MissileDamage` (`self.InstancePlayer0`)) 2.0))
  ;[1 1 1] MissileDamageEvent
  (`GameplayStatics.PlaySoundAtLocation` "/Game/MobileStarterContent/Audio/Explosion02.Explosion02" HitLocation (struct) 0.15 (`KismetMathLibrary.RandomFloatInRange` -1.0 0.3) 0.0 null null null)
  (`GameplayStatics.SpawnEmitterAtLocation` "/Game/MobileStarterContent/Particles/P_Explosion.P_Explosion" HitLocation)
  (if (>= (`KismetMathLibrary.RandomIntegerInRange` 1 9) 10)
    (bind _output_get (set `self.CurrentHealth` (- (`self.CurrentHealth`) _returnvalue)))
    (set `self.HealthPercentEnemyOne` (/ _output_get (`self.MaxHealth`)))
    (bind _returnvalue_2 (`|SpawnActorFromClass` "/Game/Stuff/UI/MissileDamageUIBP.MissileDamageUIBP_C" (`KismetMathLibrary.MakeTransform` (+ HitLocation (`KismetMathLibrary.MakeVector` (`KismetMathLibrary.RandomFloatInRange` -200.0 200.0) (`KismetMathLibrary.RandomFloatInRange` -200.0 200.0) 200.0))) "Undefined" "OverrideRootScale" null null))
    (bind _asmissile_damage_ui (cast `/Game/Stuff/UI/MissileDamageUI` (`WidgetComponent.GetUserWidgetObject` (`/Game/Stuff/UI/MissileDamageUIBP.Widget` _returnvalue_2))))
    (`TextBlock.SetText` (`/Game/Stuff/UI/MissileDamageUI.DamageText` _asmissile_damage_ui) (`KismetTextLibrary.Conv_DoubleToText` _returnvalue "HalfToEven"))
    (else
      (bind _output_get_2 (set `self.CurrentHealth` (- (`self.CurrentHealth`) (`/Game/Stuff/Instance/InstancePlayer0.MissileDamage` (`self.InstancePlayer0`)))))
      (set `self.HealthPercentEnemyOne` (/ _output_get_2 (`self.MaxHealth`)))
      (bind _returnvalue_3 (`|SpawnActorFromClass` "/Game/Stuff/UI/MissileDamageUIBP.MissileDamageUIBP_C" (`KismetMathLibrary.MakeTransform` (+ HitLocation (`KismetMathLibrary.MakeVector` (`KismetMathLibrary.RandomFloatInRange` -200.0 200.0) (`KismetMathLibrary.RandomFloatInRange` -200.0 200.0) 200.0))) "Undefined" "OverrideRootScale" null null))
      (bind _asmissile_damage_ui_2 (cast `/Game/Stuff/UI/MissileDamageUI` (`WidgetComponent.GetUserWidgetObject` (`/Game/Stuff/UI/MissileDamageUIBP.Widget` _returnvalue_3))))
      (`TextBlock.SetText` (`/Game/Stuff/UI/MissileDamageUI.DamageText` _asmissile_damage_ui_2) (`KismetTextLibrary.Conv_DoubleToText` (`/Game/Stuff/Instance/InstancePlayer0.MissileDamage` (`self.InstancePlayer0`)) "HalfToEven")))))

(event `PlasmaDamageEvent`
  (params (HitLocation :type "Vector Structure"))
  (bind _plasmamrhd (`/Game/Stuff/Instance/InstancePlayer0.PlasmaMRHD` (`self.InstancePlayer0`)))
  (bind _returnvalue (* (`/Game/Stuff/Instance/InstancePlayer0.PlasmaMRHD` (`self.InstancePlayer0`)) 2.0))
  ;[1 1 1] PlasmaDamageEvent
  (if (>= (`KismetMathLibrary.RandomIntegerInRange` 1 10) 9)
    (bind _output_get (set `self.CurrentHealth` (- (`self.CurrentHealth`) _returnvalue)))
    (set `self.HealthPercentEnemyOne` (/ _output_get (`self.MaxHealth`)))
    (bind _returnvalue_2 (`|SpawnActorFromClass` "/Game/Stuff/UI/PlasmaDamageUIBP.PlasmaDamageUIBP_C" (`KismetMathLibrary.MakeTransform` (+ HitLocation (`KismetMathLibrary.MakeVector` (`KismetMathLibrary.RandomFloatInRange` -200.0 200.0) (`KismetMathLibrary.RandomFloatInRange` -200.0 200.0) 200.0))) "Undefined" "OverrideRootScale" null null))
    (bind _asplasma_damage_ui (cast `/Game/Stuff/UI/PlasmaDamageUI` (`WidgetComponent.GetUserWidgetObject` (`/Game/Stuff/UI/PlasmaDamageUIBP.Widget` _returnvalue_2))))
    (`TextBlock.SetText` (`/Game/Stuff/UI/PlasmaDamageUI.DamageText` _asplasma_damage_ui) (`KismetTextLibrary.Conv_DoubleToText` _returnvalue "HalfToEven"))
    (else
      (bind _output_get_2 (set `self.CurrentHealth` (- (`self.CurrentHealth`) _plasmamrhd)))
      (set `self.HealthPercentEnemyOne` (/ _output_get_2 (`self.MaxHealth`)))
      (bind _returnvalue_3 (`|SpawnActorFromClass` "/Game/Stuff/UI/PlasmaDamageUIBP.PlasmaDamageUIBP_C" (`KismetMathLibrary.MakeTransform` (+ HitLocation (`KismetMathLibrary.MakeVector` (`KismetMathLibrary.RandomFloatInRange` -200.0 200.0) (`KismetMathLibrary.RandomFloatInRange` -200.0 200.0) 200.0))) "Undefined" "OverrideRootScale" null null))
      (bind _asplasma_damage_ui_2 (cast `/Game/Stuff/UI/PlasmaDamageUI` (`WidgetComponent.GetUserWidgetObject` (`/Game/Stuff/UI/PlasmaDamageUIBP.Widget` _returnvalue_3))))
      (`TextBlock.SetText` (`/Game/Stuff/UI/PlasmaDamageUI.DamageText` _asplasma_damage_ui_2) (`KismetTextLibrary.Conv_DoubleToText` _plasmamrhd "HalfToEven")))))

(event `AsteroidDamageEvent`
  (params (HitLocation :type "Vector Structure"))
  (bind _returnvalue (* (`self.MaxHealth`) 0.1))
  (bind _returnvalue_2 (* (`/Game/Stuff/Instance/InstancePlayer0.EnemyOneHealthMax` (`self.InstancePlayer0`)) 0.2))
  ;[1 1 1] AsteroidDamageEvent
  (if (>= (`KismetMathLibrary.RandomIntegerInRange` 1 10) 9)
    (bind _output_get (set `self.CurrentHealth` (- (`self.CurrentHealth`) _returnvalue_2)))
    (set `self.HealthPercentEnemyOne` (/ _output_get (`self.MaxHealth`)))
    (bind _returnvalue_3 (`|SpawnActorFromClass` "/Game/Stuff/UI/AsteroidDamageUIBP.AsteroidDamageUIBP_C" (`KismetMathLibrary.MakeTransform` (+ HitLocation (`KismetMathLibrary.MakeVector` (`KismetMathLibrary.RandomFloatInRange` -200.0 200.0) (`KismetMathLibrary.RandomFloatInRange` -200.0 200.0) 200.0))) "Undefined" "OverrideRootScale" null null))
    (bind _asasteroid_damage_ui (cast `/Game/Stuff/UI/AsteroidDamageUI` (`WidgetComponent.GetUserWidgetObject` (`/Game/Stuff/UI/AsteroidDamageUIBP.Widget` _returnvalue_3))))
    (`TextBlock.SetText` (`/Game/Stuff/UI/AsteroidDamageUI.DamageText` _asasteroid_damage_ui) (`KismetTextLibrary.Conv_DoubleToText` _returnvalue_2 "HalfToEven"))
    (else
      (bind _output_get_2 (set `self.CurrentHealth` (- (`self.CurrentHealth`) _returnvalue)))
      (set `self.HealthPercentEnemyOne` (/ _output_get_2 (`/Game/Stuff/Instance/InstancePlayer0.EnemyOneHealthMax` (`self.InstancePlayer0`))))
      (bind _returnvalue_4 (`|SpawnActorFromClass` "/Game/Stuff/UI/AsteroidDamageUIBP.AsteroidDamageUIBP_C" (`KismetMathLibrary.MakeTransform` (+ HitLocation (`KismetMathLibrary.MakeVector` (`KismetMathLibrary.RandomFloatInRange` -200.0 200.0) (`KismetMathLibrary.RandomFloatInRange` -200.0 200.0) 200.0))) "Undefined" "OverrideRootScale" null null))
      (bind _asasteroid_damage_ui_2 (cast `/Game/Stuff/UI/AsteroidDamageUI` (`WidgetComponent.GetUserWidgetObject` (`/Game/Stuff/UI/AsteroidDamageUIBP.Widget` _returnvalue_4))))
      (`TextBlock.SetText` (`/Game/Stuff/UI/AsteroidDamageUI.DamageText` _asasteroid_damage_ui_2) (`KismetTextLibrary.Conv_DoubleToText` _returnvalue "HalfToEven")))))

(fn `CalculateLaunchVelocity`
  (params (Actor :type "Actor Object Reference"))
  (returns (Output_Get :type "Vector Structure"))
  (bind (_returnvalue_x _returnvalue_y _returnvalue_z) (`KismetMathLibrary.BreakVector` (`KismetMathLibrary.GetDirectionUnitVector` (`self.K2_GetActorLocation` Actor) (`self.K2_GetActorLocation`))))
  (bind (_returnvalue_x_2 _returnvalue_y_2 _returnvalue_z_2) (`KismetMathLibrary.BreakVector` (* (`KismetMathLibrary.MakeVector` _returnvalue_x _returnvalue_y _returnvalue_z) (`self.LaunchVelocity`))))
  (bind _output_get (set `self.CurrentLaunch` (`KismetMathLibrary.ClampVectorSize` (`KismetMathLibrary.MakeVector` (* _returnvalue_x_2 2.0) (* _returnvalue_y_2 2.0) (`KismetMathLibrary.FClamp` (+ _returnvalue_z_2 (`self.LaunchHeight`)) 400.0 700.0)) 0.0 500.0)))
  (return _output_get))

(fn `UserConstructionScript`)