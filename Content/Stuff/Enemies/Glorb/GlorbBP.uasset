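; GlorbBP is the Glorb enemy Blueprint, which only animates the scale of its big eye, small eye and body.
; On BeginPlay, three timelines each lerp one component between a smaller and larger uniform scale.
; They are chained through Update pins with short Delays, so the small eye's animation starts after the big eye's and the body's follows, staggering the motion.
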(event `self.ReceiveBeginPlay`
  (bind (_direction _newtrack_0) (`Timeline|Timeline_0`)
    (:`Update`
      (`SceneComponent.SetRelativeScale3D` (`self.BigEye`) (`KismetMathLibrary.VLerp` (0.3 0.3 0.3) (0.7 0.7 0.7) _newtrack_0))
      (`KismetSystemLibrary.Delay` 0.2)
      (bind (_direction_2 _newtrack_0_2) (`Timeline|Timeline_1`)
        (:`Update`
          (`SceneComponent.SetRelativeScale3D` (`self.SmallEye`) (`KismetMathLibrary.VLerp` (0.2 0.2 0.2) (0.4 0.4 0.4) _newtrack_0_2))
          (`KismetSystemLibrary.Delay` 0.2)
          (bind (_direction_3 _newtrack_0_3) (`Timeline|Timeline_2`)
            (:`Update`
              (`SceneComponent.SetRelativeScale3D` (`self.GlorbBody`) (`KismetMathLibrary.VLerp` (0.2 0.2 0.2) (0.25 0.25 0.25) _newtrack_0_3)))))))))

(fn `UserConstructionScript`)