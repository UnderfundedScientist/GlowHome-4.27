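; Brain pickup drop that triggers a level-up on the twin-stick player pawn when collected.
; On BeginPlay it caches the player and game instance (the latter unused here), animates the mesh scale with a timeline, and starts a 30-second self-destruct timer.
; Player overlap with the pickup radius calls the pawn's LevelUpEvent, plays a click sound and destroys the actor.
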(event `self.ReceiveBeginPlay`
  (`|ExecutionSequence`
    (:`then_0`
      (`self.CastEvent`))
    (:`then_1`
      (bind (_direction _newtrack_0) (`Timeline|Timeline_0`)
        (:`Update`
          (`SceneComponent.SetRelativeScale3D` (`self.StaticMesh`) (`KismetMathLibrary.VLerp` (0.5 0.5 0.5) (1.2 1.2 1.2) _newtrack_0)))))
    (:`then_2`
      (`KismetSystemLibrary.K2_SetTimer` null "DeathClock" 30.0))))

(event `CastEvent`
  (`|ExecutionSequence`
    (:`then_0`
      (bind _astwin_stick_pawn (cast `/Game/Stuff/TwinStickBP/Blueprints/TwinStickPawn` (`GameplayStatics.GetPlayerPawn` 0)))
      (set `self.Player` _astwin_stick_pawn))
    (:`then_1`
      (bind _asinstance_player_0 (cast `/Game/Stuff/Instance/InstancePlayer0` (`GameplayStatics.GetGameInstance`)))
      (set `self.Instance` _asinstance_player_0))))

(event `self.PickupRadius.OnComponentBeginOverlap`
  (params (OverlappedComponent :type "PrimitiveComponent Object Reference") (OtherActor :type "Actor Object Reference") (OtherComp :type "PrimitiveComponent Object Reference") (OtherBodyIndex :type Integer) (bFromSweep :type Boolean) (SweepResult :type "HitResult Structure (by ref)"))
  (if (== OtherActor (`self.Player`))
    (`self.BrainPickupEvent`)))

(event `BrainPickupEvent`
  (`/Game/Stuff/TwinStickBP/Blueprints/TwinStickPawn.LevelUpEvent` (`self.Player`))
  (`GameplayStatics.PlaySoundAtLocation` "/Game/Stuff/Sounds/MenuClick.MenuClick" (`self.K2_GetActorLocation`) (struct) 1.0 1.0 0.0 null null null)
  (`self.K2_DestroyActor`))

(event `DeathClock`
  (`self.K2_DestroyActor`))

(fn `UserConstructionScript`)