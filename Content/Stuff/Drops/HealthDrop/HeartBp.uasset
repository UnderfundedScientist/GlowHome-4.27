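; Health drop pickup for the twin-stick player that restores 30% of max health on overlap with its pickup radius.
; On begin play it caches the player pawn and game instance, where health is stored.
; Pickup updates the stored health without clamping to the max, pushes the percentage to the player's health bar material, plays a sound and destroys itself.
; An uncollected drop destroys itself after a 30-second timer.
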(event `self.ReceiveBeginPlay`
  (`|ExecutionSequence`
    (:`then_0`
      (`self.CastEvent`))
    (:`then_2`
      (`KismetSystemLibrary.K2_SetTimer` null "DeathClock" 30.0))))

(event `CastEvent`
  (`|ExecutionSequence`
    (:`then_0`
      (bind _astwin_stick_pawn (cast `/Game/Stuff/Player/Blueprints/TwinStickPawn` (`GameplayStatics.GetPlayerPawn` 0)))
      (set `self.Player` _astwin_stick_pawn))
    (:`then_1`
      (bind _asinstance_player_0 (cast `/Game/Stuff/Instance/InstancePlayer0` (`GameplayStatics.GetGameInstance`)))
      (set `self.Instance` _asinstance_player_0))))

(event `self.PickupRadius.OnComponentBeginOverlap`
  (params (OverlappedComponent :type "PrimitiveComponent Object Reference") (OtherActor :type "Actor Object Reference") (OtherComp :type "PrimitiveComponent Object Reference") (OtherBodyIndex :type Integer) (bFromSweep :type Boolean) (SweepResult :type "HitResult Structure (by ref)"))
  (if (== OtherActor (`self.Player`))
    (`self.HealthPickupEvent`)))

(event `HealthPickupEvent`
  (bind _instance (`self.Instance`))
  (bind _playerhealthmaxinstance (`/Game/Stuff/Instance/InstancePlayer0.PlayerHealthMaxInstance` _instance))
  (bind _output_get (set `/Game/Stuff/Instance/InstancePlayer0.PlayerHealthInstance` (+ (`/Game/Stuff/Instance/InstancePlayer0.PlayerHealthInstance` _instance) (* _playerhealthmaxinstance 0.3)) _instance))
  (bind _output_get_2 (set `/Game/Stuff/Instance/InstancePlayer0.PlayerHealthPercentInstance` (/ _output_get _playerhealthmaxinstance) _instance))
  (`MeshComponent.SetScalarParameterValueOnMaterials` (`/Game/Stuff/Player/Blueprints/TwinStickPawn.HealthBarPlane` (`self.Player`)) "HealthPercent" _output_get_2)
  (`GameplayStatics.PlaySoundAtLocation` "/Game/Stuff/Sounds/MenuClick.MenuClick" (`self.K2_GetActorLocation`) (struct) 1.0 1.0 0.0 null null null)
  (`self.K2_DestroyActor`))

(event `DeathClock`
  (`self.K2_DestroyActor`))

(fn `UserConstructionScript`)