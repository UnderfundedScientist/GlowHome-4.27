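; Gold bar drop that homes in on the player and awards gold when collected.
; On BeginPlay it gets a random rotating-movement spin and caches the TwinStickPawn player and InstancePlayer0 game instance.
; MagnetRadius uses AIMoveTo to pull the bar toward the player, either on overlap or when already inside at spawn.
; A capsule hit or overlap with the player adds RewardGold to GoldInstance on the game instance and destroys the bar.
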(event `self.ReceiveBeginPlay`
  (`|ExecutionSequence`
    (:`then_0`
      (set `RotatingMovementComponent.PivotTranslation` (`KismetMathLibrary.RandomUnitVector`) (`self.RotatingMovement`))
      (set `RotatingMovementComponent.RotationRate` (`KismetMathLibrary.RandomRotator` true) (`self.RotatingMovement`)))
    (:`then_1`
      (bind _astwin_stick_pawn (cast `/Game/Stuff/Player/Blueprints/TwinStickPawn` (`GameplayStatics.GetPlayerPawn` 0)))
      (set `self.Player` _astwin_stick_pawn))
    (:`then_2`
      (bind _asinstance_player_0 (cast `/Game/Stuff/Instance/InstancePlayer0` (`GameplayStatics.GetGameInstance`)))
      (set `self.As Instance Player 0` _asinstance_player_0))
    (:`then_3`
      (if (`PrimitiveComponent.IsOverlappingActor` (`self.MagnetRadius`) (`self.Player`))
        (`AITask_MoveTo.AIMoveTo` (`AIBlueprintHelperLibrary.GetAIController` self) (0.0 0.0 0.0) (`self.Player`))))))

(event `self.MagnetRadius.OnComponentBeginOverlap`
  (params (OverlappedComponent :type "PrimitiveComponent Object Reference") (OtherActor :type "Actor Object Reference") (OtherComp :type "PrimitiveComponent Object Reference") (OtherBodyIndex :type Integer) (bFromSweep :type Boolean) (SweepResult :type "HitResult Structure (by ref)"))
  (if (== OtherActor (`self.Player`))
    (`|AIMoveTo` self (0.0 0.0 0.0) (`self.Player`) 0.0)))

(event `self.CapsuleComponent.OnComponentHit`
  (params (HitComponent :type "PrimitiveComponent Object Reference") (OtherActor :type "Actor Object Reference") (OtherComp :type "PrimitiveComponent Object Reference") (NormalImpulse :type "Vector Structure") (Hit :type "HitResult Structure (by ref)"))
  (bind _as_instance_player_0 (`self.As Instance Player 0`))
  (if (== OtherActor (`self.Player`))
    (set `/Game/Stuff/Instance/InstancePlayer0.GoldInstance` (+ (`/Game/Stuff/Instance/InstancePlayer0.GoldInstance` _as_instance_player_0) (`/Game/Stuff/Instance/InstancePlayer0.RewardGold` _as_instance_player_0)) _as_instance_player_0)
    (`self.K2_DestroyActor`)))

(event `self.CapsuleComponent.OnComponentBeginOverlap`
  (params (OverlappedComponent :type "PrimitiveComponent Object Reference") (OtherActor :type "Actor Object Reference") (OtherComp :type "PrimitiveComponent Object Reference") (OtherBodyIndex :type Integer) (bFromSweep :type Boolean) (SweepResult :type "HitResult Structure (by ref)"))
  (bind _as_instance_player_0 (`self.As Instance Player 0`))
  (if (== OtherActor (`self.Player`))
    (set `/Game/Stuff/Instance/InstancePlayer0.GoldInstance` (+ (`/Game/Stuff/Instance/InstancePlayer0.GoldInstance` _as_instance_player_0) (`/Game/Stuff/Instance/InstancePlayer0.RewardGold` _as_instance_player_0)) _as_instance_player_0)
    (`self.K2_DestroyActor`)))

(fn `UserConstructionScript`)